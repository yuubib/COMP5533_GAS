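; Enemy character Blueprint that handles hit feedback, death, stun and knockback for an AI-controlled opponent.
; HP changes update the overhead bar from a GAS attribute, play a sound and hit montage with brief slow-motion, then on death play a montage and stop AI logic.
; Stun pauses BP_AIController's brain for a duration, while PushAlway applies an impulse with friction temporarily zeroed during a montage.
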(event `self.HPChangeEvent_Event`
  (params (NewValue :type "Float (single-precision)"))
  (`parent.HPChangeEvent_Event` NewValue)
  (`/Game/BP/UMG/UMG_EnemyBar.SetPer` (cast `/Game/BP/UMG/UMG_EnemyBar` (`WidgetComponent.GetUserWidgetObject` (`self.HPBar`)) :!pure true) (/ NewValue (`.ReturnValue` (`AbilitySystemBlueprintLibrary.GetFloatAttributeFromAbilitySystemComponent` (`self.AbilitySystem`) (struct :`AttributeName` "MaxHP" :`Attribute` "/Script/comp5533_GAS.BaseAttributeSet:MaxHP" :`AttributeOwner` "/Script/CoreUObject.Class'/Script/comp5533_GAS.BaseAttributeSet'")))))
  (`GameplayStatics.PlaySound2D` "/Engine/EditorSounds/GamePreview/EndSimulate.EndSimulate" 1.0 1.0 0.0 null null)
  (`GameplayStatics.SetGlobalTimeDilation` 0.4)
  (`self.PlayAnimMontage` "/Game/Ani/Montage/MA_Hit.MA_Hit")
  (`KismetSystemLibrary.Delay` 0.1)
  (`GameplayStatics.SetGlobalTimeDilation` 1.0)
  (if (`self.IsDeath`)
    (`self.PlayAnimMontage` "/Game/Ani/Montage/MA_Death.MA_Death")
    (`self.StopController`)))

(event `Stun`
  (params (StartDuration :type "Float (double-precision)"))
  (`self.StopController`)
  (`KismetSystemLibrary.Delay` StartDuration)
  (`self.ResetControll`))

(event `PushAlway`
  (params (AnimMontage :type "AnimMontage Object Reference") (ImpulseDir :type "Vector Structure") (Strength :type "Float (single-precision)") (DurationTime :type "Float (single-precision)"))
  (`|PlayMontage` null AnimMontage
    (:`then`
      (`self.SetFrictionToZero` true)
      (`CharacterMovementComponent.AddImpulse` (`self.CharacterMovement`) (* ImpulseDir Strength) true)
      (`KismetSystemLibrary.Delay` DurationTime)
      (`self.SetFrictionToZero` false))))

(fn `ResetControll`
  (bind _asbp_aicontroller (cast `/Game/BP/Character/AI/00Enemy/BP_AIController` (`self.GetController`)))
  (`BrainComponent.RestartLogic` (`AIController.BrainComponent` _asbp_aicontroller)))

(fn `StopController`
  (bind _asbp_aicontroller (cast `/Game/BP/Character/AI/00Enemy/BP_AIController` (`self.GetController`)))
  (`BrainComponent.StopLogic` (`AIController.BrainComponent` _asbp_aicontroller) "Death"))

(fn `UserConstructionScript`
  (`parent.UserConstructionScript`))