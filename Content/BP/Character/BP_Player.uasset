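; Player character Blueprint built on the Gameplay Ability System, with a lockable camera and abilities activated by tag through an index.
; On BeginPlay it activates a regen ability, grants its ability list and fills the matching UI slots.
; Attribute change events update HP, MP and Strength bars on the controller's MainUI, and death disables input.
; Sphere overlaps with enemies send a Dash gameplay event to itself, carrying the enemy as target.
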(event `self.ReceiveBeginPlay`
  (`parent.ReceiveBeginPlay`)
  (`|ExecutionSequence`
    (:`then_0`
      (bind _asbp_player_controller (cast `/Game/BP/Gameplay/BP_PlayerController` (`GameplayStatics.GetPlayerController` 0)))
      (set `self.As BP Player Controller` _asbp_player_controller))
    (:`then_1`
      (`AbilitySystemComponent.K2_GiveAbilityAndActivateOnce` (`self.AbilitySystem`) "/Game/BP/Ability/BaseRegen/BP_BaseRegen.BP_BaseRegen_C" 0 -1))
    (:`then_2`
      (for (_array_element _array_index) (`self.GABs`)
        (`AbilitySystemComponent.K2_GiveAbility` (`self.AbilitySystem`) _array_element 0 -1)
        (bind _returnvalue (`self.GameplayAbilityInfo` _array_element))
        (`self.InitUIinput` _returnvalue _array_index)))
    (:`then_3`
      (add `self.MPChangeEvent` (delegate `MPChangeEvent_Event`))
      (add `self.StrengthChangeEvent` (delegate `StrengthChangeEvent_Event`)))))

(event `MPChangeEvent_Event` :!signature `self.MPChangeEvent`
  (params (NewValue :type "Float (single-precision)"))
  (`/Game/BP/UMG/UMG_AttributeBar.SetPer` (`/Game/BP/UMG/UMG_MainUI.UMGAttributeBar_MP` (`/Game/BP/Gameplay/BP_PlayerController.MainUI` (`.AsBP Player Controller` (`/Game/BP/BPF_Lib.GetPlayerAndContro`)))) (/ NewValue (`.ReturnValue` (`AbilitySystemBlueprintLibrary.GetFloatAttributeFromAbilitySystemComponent` (`self.AbilitySystem`) (struct :`AttributeName` "MaxMP" :`Attribute` "/Script/comp5533_GAS.BaseAttributeSet:MaxMP" :`AttributeOwner` "/Script/CoreUObject.Class'/Script/comp5533_GAS.BaseAttributeSet'"))))))

(event `StrengthChangeEvent_Event` :!signature `self.StrengthChangeEvent`
  (params (NewValue :type "Float (single-precision)"))
  (`/Game/BP/UMG/UMG_AttributeBar.SetPer` (`/Game/BP/UMG/UMG_MainUI.UMGAttributeBar_Strenght` (`/Game/BP/Gameplay/BP_PlayerController.MainUI` (`.AsBP Player Controller` (`/Game/BP/BPF_Lib.GetPlayerAndContro`)))) (/ NewValue (`.ReturnValue` (`AbilitySystemBlueprintLibrary.GetFloatAttributeFromAbilitySystemComponent` (`self.AbilitySystem`) (struct :`AttributeName` "MaxStrength" :`Attribute` "/Script/comp5533_GAS.BaseAttributeSet:MaxStrength" :`AttributeOwner` "/Script/CoreUObject.Class'/Script/comp5533_GAS.BaseAttributeSet'"))))))

(event `self.ReceiveTick`
  (params (DeltaSeconds :type "Float (single-precision)")))

(event `self.HPChangeEvent_Event`
  (params (NewValue :type "Float (single-precision)"))
  (`parent.HPChangeEvent_Event` NewValue)
  (`/Game/BP/UMG/UMG_AttributeBar.SetPer` (`/Game/BP/UMG/UMG_MainUI.UMGAttributeBar_HP` (`/Game/BP/Gameplay/BP_PlayerController.MainUI` (`self.As BP Player Controller`))) (/ NewValue (`.ReturnValue` (`AbilitySystemBlueprintLibrary.GetFloatAttributeFromAbilitySystemComponent` (`self.AbilitySystem`) (struct :`AttributeName` "MaxHP" :`Attribute` "/Script/comp5533_GAS.BaseAttributeSet:MaxHP" :`AttributeOwner` "/Script/CoreUObject.Class'/Script/comp5533_GAS.BaseAttributeSet'")))))
  (if (`self.IsDeath`)
    (`self.DisableInput` (`self.As BP Player Controller`) null)))

(event `self.Sphere.OnComponentBeginOverlap`
  (params (OverlappedComponent :type "PrimitiveComponent Object Reference") (OtherActor :type "Actor Object Reference") (OtherComp :type "PrimitiveComponent Object Reference") (OtherBodyIndex :type Integer) (bFromSweep :type Boolean) (SweepResult :type "HitResult Structure (by ref)"))
  (`KismetArrayLibrary.Array_Clear` (`self.As Enemy`))
  (bind _asbp_enemy (cast `/Game/BP/Character/BP_Enemy` OtherActor))
  (if (not (`KismetArrayLibrary.Array_Contains` (`self.As Enemy`) _asbp_enemy))
    (`KismetArrayLibrary.Array_AddUnique` (`self.As Enemy`) _asbp_enemy)
    (`AbilitySystemBlueprintLibrary.SendGameplayEventToActor` self (struct :`TagName` "Ability.Dash.Event") (make `GameplayEventData` (struct :`TagName` "Ability.Dash.Event") self _asbp_enemy))))

(fn `ActiveAbility_My`
  (params (Index :type Integer))
  (`AbilitySystemComponent.TryActivateAbilitiesByTag` (`self.AbilitySystem`) (`|GetArrayItem` (`self.Gameplay Tag Container_0`) Index) true))

(fn `HPIsFull`
  (returns (`Full?` :type Boolean))
  (return (>= (`.ReturnValue` (`AbilitySystemBlueprintLibrary.GetFloatAttributeFromAbilitySystemComponent` (`self.AbilitySystem`) (struct :`AttributeName` "HP" :`Attribute` "/Script/comp5533_GAS.BaseAttributeSet:HP" :`AttributeOwner` "/Script/CoreUObject.Class'/Script/comp5533_GAS.BaseAttributeSet'"))) 100.0)))

(fn `InitUIinput`
  (params (AbilityInfo :type "MyGameplayAbilityInfo Structure") (`Dimension 1` :type Integer))
  (`/Game/BP/UMG/UMG_AbilitySlot.CE_InitInfo` (`|GetArrayItem` (`/Game/BP/UMG/UMG_MainUI.UMGAbilityAll` (`/Game/BP/Gameplay/BP_PlayerController.MainUI` (`.AsBP Player Controller` (`/Game/BP/BPF_Lib.GetPlayerAndContro`)))) `Dimension 1`) AbilityInfo))

(fn `LockCamera`
  (params (isLock :type Boolean))
  (bind _springarm (`self.SpringArm`))
  (bind _charactermovement (`self.CharacterMovement`))
  (bind _camera (`self.Camera`))
  (if isLock
    (set `self.bUseControllerRotationYaw` true)
    (set `SpringArmComponent.bUsePawnControlRotation` false _springarm)
    (set `CharacterMovementComponent.bOrientRotationToMovement` false _charactermovement)
    (`SceneComponent.K2_SetRelativeLocationAndRotation` _camera (0.0 0.0 200.0) (struct :`Pitch` -20.0) true false)
    (else
      (set `self.bUseControllerRotationYaw` false)
      (set `SpringArmComponent.bUsePawnControlRotation` true _springarm)
      (set `CharacterMovementComponent.bOrientRotationToMovement` true _charactermovement)
      (`SceneComponent.K2_SetRelativeLocationAndRotation` :`self` _camera :`bSweep` true))))

(fn `MPIsFull`
  (returns (`Full?` :type Boolean))
  (return (>= (`.ReturnValue` (`AbilitySystemBlueprintLibrary.GetFloatAttributeFromAbilitySystemComponent` (`self.AbilitySystem`) (struct :`AttributeName` "MP" :`Attribute` "/Script/comp5533_GAS.BaseAttributeSet:MP" :`AttributeOwner` "/Script/CoreUObject.Class'/Script/comp5533_GAS.BaseAttributeSet'"))) 100.0)))

(fn `UserConstructionScript`
  (`parent.UserConstructionScript`))