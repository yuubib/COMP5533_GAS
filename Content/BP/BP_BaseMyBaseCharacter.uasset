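; Base character Blueprint built on the Gameplay Ability System, providing a melee ability and contact damage between characters.
; BeginPlay grants GAB_Melee, and the Melee event activates it through a helper that looks up gameplay tags by index.
; DamageCapsule overlaps apply GE_Melee_Damage at a random level to other base-derived characters of a different class, skipping same-class ones.
; The hit target then prints an attribute value for debugging.
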(event `self.ReceiveBeginPlay`
  (`AbilitySystemComponent.K2_GiveAbility` (`self.AbilitySystem`) "/Game/BP/Ability/00Melee/GAB_Melee.GAB_Melee_C" 0 -1)
  (`KismetSystemLibrary.PrintString` "Hello"))

(event `Melee`
  ; 技能觸發
  (`self.ActivateAbility` 0))

(event `self.DamageCapsule.OnComponentBeginOverlap`
  (params (OverlappedComponent :type "PrimitiveComponent Object Reference") (OtherActor :type "Actor Object Reference") (OtherComp :type "PrimitiveComponent Object Reference") (OtherBodyIndex :type Integer) (bFromSweep :type Boolean) (SweepResult :type "HitResult Structure (by ref)"))
  (if (and (!= OtherActor self) (!= (`GameplayStatics.GetObjectClass` OtherActor) (`GameplayStatics.GetObjectClass` self)))
    (bind _asbp_base_my_base_character (cast `/Game/BP/BP_BaseMyBaseCharacter` OtherActor))
    (`AbilitySystemComponent.BP_ApplyGameplayEffectToTarget` :`self` (`self.AbilitySystem`) :`GameplayEffectClass` "/Game/BP/Ability/00Melee/GE_Melee_Damage.GE_Melee_Damage_C" :`Target` (`/Game/BP/BP_BaseMyBaseCharacter.AbilitySystem` _asbp_base_my_base_character) :`Level` (`KismetMathLibrary.Conv_IntToDouble` (`KismetMathLibrary.RandomInteger` 2)))
    (`self.ShowAttribute` _asbp_base_my_base_character (struct :`AttributeName` "HP" :`Attribute` "/Script/comp5533_GAS.BaseAttributeSet:HP" :`AttributeOwner` "/Script/CoreUObject.Class'/Script/comp5533_GAS.BaseAttributeSet'"))))

(event `ShowAttribute`
  (params (Attribute :type "GameplayAttribute Structure"))
  (`KismetSystemLibrary.PrintString` (`KismetStringLibrary.Conv_DoubleToString` (`.ReturnValue` (`AbilitySystemBlueprintLibrary.GetFloatAttributeFromAbilitySystemComponent` (`self.AbilitySystem`) Attribute)))))

(fn `ActivateAbility`
  (params (AbilityIndex :type Integer))
  (`AbilitySystemComponent.TryActivateAbilitiesByTag` (`self.AbilitySystem`) (`|GetArrayItem` (`self.Gameplay Tag Container`) AbilityIndex) true))

(fn `UserConstructionScript`)